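; Spiderling enemy Blueprint that self-detonates when the player enters its detonation sphere.
; The construction script sizes the sphere from DetonationRadius, then runs the parent construction script.
; On overlap with bpPlayer, it attaches the particle effect and sound to the player's CenterPoint, triggers a camera shake and destroys itself.
; The graph itself applies no damage.
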(event OnComponentBeginOverlap(DetonationSphere)
  (params (OverlappedComponent :type Primitive%20Component%20Object%20Reference) (OtherActor :type Actor%20Object%20Reference) (OtherComp :type Primitive%20Component%20Object%20Reference) (OtherBodyIndex :type Integer) (bFromSweep :type Boolean) (SweepResult :type Hit%20Result%20Structure%20%28by%20ref%29))
  ;[1 1 1] Detonation effect
  (bind _asbp_player (Utilities|Casting|CastTobpPlayer OtherActor))
  (Variables|Default|SetPlayerRef _asbp_player)
  (Effects|SpawnEmitterAttached (Variables|UltraForce-Explodite|GetPE_OnPlayerAfterDetonation) (Variables|/Game/Blueprints/Misc/bpPlayer.bpPlayer_C|GetCenterPoint (Variables|Default|GetPlayerRef)) "" (Transformation|GetActorLocation (Variables|Default|GetPlayerRef)) "90.000000, 0, 0" "KeepWorldPosition")
  (Default|CameraShake (Variables|Default|GetPlayerRef) (Variables|UltraForce-Explodite|GetCameraShakeClass) (Variables|UltraForce-Explodite|GetCameraShakeScale))
  (Audio|SpawnSoundAttached (Variables|UltraForce-Explodite|GetDetonationSound) (Variables|/Game/Blueprints/Misc/bpPlayer.bpPlayer_C|GetCenterPoint (Variables|Default|GetPlayerRef)) "None" "0, 0, 0" "0, 0, 0" "KeepRelativeOffset" false 1.0 1.0 0.8)
  (Actor|DestroyActor))

(event EventBeginPlay)

(event Collision|EventActorBeginOverlap
  (params (OtherActor :type Actor%20Object%20Reference)))

(event EventTick
  (params (DeltaSeconds :type Float%20%28single-precision%29)))

(fn ConstructionScript
  (Components|Sphere|SetSphereRadius (Variables|Default|GetDetonationSphere) (Variables|UltraForce-Explodite|GetDetonationRadius) true)
  (|CallParentFunction))