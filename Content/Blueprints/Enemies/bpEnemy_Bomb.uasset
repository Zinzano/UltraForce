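; bpEnemy_Bomb is an enemy that telegraphs a strike on a locked player position, using particles, sounds and camera shake.
; HomingInOnPlayer plays warning effects, then stores the player's location after a delay.
; FireAtLockedPlayerLocation plays a firing sound, then after a delay shows the impact there and shakes the camera, applying no damage.
; Nothing here calls either event; aggro overlaps trigger nothing, and the older AttackPlayer sequence is disconnected.
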(event OnComponentBeginOverlap(AggroSphere)
  (params (OverlappedComponent :type Primitive%20Component%20Object%20Reference) (OtherActor :type Actor%20Object%20Reference) (OtherComp :type Primitive%20Component%20Object%20Reference) (OtherBodyIndex :type Integer) (bFromSweep :type Boolean) (SweepResult :type Hit%20Result%20Structure%20%28by%20ref%29))
  ;[1 1 1] Comment
)

(event OnComponentEndOverlap(AggroSphere)
  (params (OverlappedComponent :type Primitive%20Component%20Object%20Reference) (OtherActor :type Actor%20Object%20Reference) (OtherComp :type Primitive%20Component%20Object%20Reference) (OtherBodyIndex :type Integer))
  (Utilities|Casting|CastTobpPlayer OtherActor))

(event Custom|AttackPlayer
  (params (PlayerRef :type Bp%20Player%20Object%20Reference))
  ;[1 1 1] NOT IN USE
)

(event Custom|HomingInOnPlayer
  (params (PlayerRef :type Bp%20Player%20Object%20Reference))
  (bind _bottompoint (Variables|Default|GetBottomPoint))
  (bind _returnvalue (Transformation|GetWorldLocation _bottompoint))
  ;[1 1 1] Comment
  (Effects|SpawnEmitteratLocation (Variables|Default|GetPE_HomingInOnPlayer) (Math|Vector|MakeVector (.x _returnvalue) (.y _returnvalue) (.z _returnvalue)))
  (Audio|SpawnSoundatLocation (Variables|Default|GetSound_HomingInOnPlayer) (Transformation|GetActorLocation))
  (Utilities|FlowControl|Delay 2.5)
  (Variables|Default|SetLockedPlayerLocation (Transformation|GetActorLocation PlayerRef)))

(event Custom|FireAtLockedPlayerLocation
  (params (PlayerRef :type Bp%20Player%20Object%20Reference))
  (bind _lockedplayerlocation (Variables|Default|GetLockedPlayerLocation))
  ;[1 1 1] Comment
  (Audio|PlaySoundatLocation (Variables|Default|GetSound_FireAtPlayer) (Transformation|GetActorLocation))
  (Utilities|FlowControl|Delay 1.0)
  (Effects|SpawnEmitteratLocation (Variables|Default|GetPE_WeaponHit) (Math|Vector|MakeVector (- (.x _lockedplayerlocation) -5e+01) (.y _lockedplayerlocation) (- (.z _lockedplayerlocation) 5e+01)))
  (Default|CameraShake PlayerRef "/Game/Blueprints/Misc/CameraShake/bpCameraShakeShort.bpCameraShakeShort_C" 22.0)
  (Audio|PlaySoundatLocation (Variables|Default|GetSound_WeaponHit) (Variables|Default|GetLockedPlayerLocation)))

(event EventBeginPlay)

(event Collision|EventActorBeginOverlap
  (params (OtherActor :type Actor%20Object%20Reference)))

(event EventTick
  (params (DeltaSeconds :type Float%20%28single-precision%29)))

(fn ConstructionScript
  (|CallParentFunction))