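; Enemy turret Blueprint that turns toward the player pawn and fires projectiles while its aggro sphere is triggered.
; Any overlap with the sphere, sized from AggroRange at construction, starts a looping Fire timer and opens a Tick gate; ending overlap stops both.
; The gated Tick smoothly interpolates the turret toward the player, and Fire spawns a half-scale projectile at the turret's transform.
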(event OnComponentBeginOverlap(AggroRadius)
  (params (OverlappedComponent :type Primitive%20Component%20Object%20Reference) (OtherActor :type Actor%20Object%20Reference) (OtherComp :type Primitive%20Component%20Object%20Reference) (OtherBodyIndex :type Integer) (bFromSweep :type Boolean) (SweepResult :type Hit%20Result%20Structure%20%28by%20ref%29))
  (bind _turret (Variables|Default|GetTurret))
  (Utilities|Time|SetTimerbyFunctionName 0 "Fire" (Variables|UltraForce-Turret|GetReloadTime) true)
  (Utilities|FlowControl|Gate true) ; enters at Open
)

(event OnComponentEndOverlap(AggroRadius)
  (params (OverlappedComponent :type Primitive%20Component%20Object%20Reference) (OtherActor :type Actor%20Object%20Reference) (OtherComp :type Primitive%20Component%20Object%20Reference) (OtherBodyIndex :type Integer))
  (bind _turret (Variables|Default|GetTurret))
  (Utilities|Time|ClearTimerbyFunctionName 0 "Fire")
  (Utilities|FlowControl|Gate true) ; enters at Close
)

(event Custom|Fire
  (bind _turret (Variables|Default|GetTurret))
  (bind _returnvalue (Transformation|GetWorldTransform _turret))
  (Game|SpawnActorfromClass (Variables|Default|GetProjectileClass) (Math|Transform|MakeTransform (.location _returnvalue) (.rotation _returnvalue) "0.500000,0.500000,0.500000") "AlwaysSpawn" 0 0))

(event EventBeginPlay)

(event Collision|EventActorBeginOverlap
  (params (OtherActor :type Actor%20Object%20Reference)))

(event EventTick
  (params (DeltaSeconds :type Float%20%28single-precision%29))
  (bind _turret (Variables|Default|GetTurret))
  (Utilities|FlowControl|Gate true
    (:Exit
      (Transformation|SetWorldRotation _turret (Math|Interpolation|RInterpTo (Transformation|GetWorldRotation _turret) (Math|Rotator|FindLookatRotation (Transformation|GetWorldLocation _turret) (Transformation|GetActorLocation (Game|Player|GetPlayerPawn 0))) DeltaSeconds (Variables|UltraForce-Turret|GetTurretRotSpeed)) false false))))

(fn ConstructionScript
  (Components|Sphere|SetSphereRadius (Variables|Default|GetAggroRadius) (Variables|UltraForce-Turret|GetAggroRange) true))