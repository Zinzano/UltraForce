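; Base enemy Blueprint that handles health, death and patrol-route bookkeeping.
; Damage lowers clamped health, and at zero the enemy spawns a death particle, plays a sound and destroys itself.
; The construction script sizes the aggro sphere from AggroRange.
; Helper functions return the current patrol point's location and advance the index, either looping or ping-ponging along the path when ReversePatrolPathWhenDone is set.
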(event EventBeginPlay
  (Variables|Default|SetHealth (Variables|Default|GetMaxHealth)))

(event Collision|EventActorBeginOverlap
  (params (OtherActor :type Actor%20Object%20Reference)))

(event Game|Damage|EventAnyDamage
  (params (Damage :type Float%20%28single-precision%29) (DamageType :type Damage%20Type%20Object%20Reference) (InstigatedBy :type Controller%20Object%20Reference) (DamageCauser :type Actor%20Object%20Reference))
  (Variables|Default|SetHealth (Math|Float|Clamp(Float) (- (Variables|Default|GetHealth) Damage) 0.0 (Variables|Default|GetMaxHealth)))
  (if (<= (Variables|Default|GetHealth) 0.0)
    (Effects|SpawnEmitteratLocation (Variables|Default|GetPE_Death) (Transformation|GetWorldLocation (Variables|Default|GetBottomPoint)))
    (Audio|PlaySoundatLocation (Variables|Default|GetDeathSound) (Transformation|GetActorLocation) "0, 0, 0" 1.0 1.0 1.0)
    (Actor|DestroyActor)))

(event EventTick
  (params (DeltaSeconds :type Float%20%28single-precision%29)))

(fn ConstructionScript
  (Components|Sphere|SetSphereRadius (Variables|Default|GetAggroSphere) (Variables|Default|GetAggroRange) true))

(fn GetCurrentPatrolPoint
  (return (Transformation|GetActorLocation (Utilities|Array|Get(acopy) (Variables|Default|GetPatrolPoints) (Variables|Default|GetPatrolPointIndex)))))

(fn IncrementPatrolPointIndex
  ;[1 1 1] IncrementPatrolPointIndex
  ;;[1 1 1] Are we at the last PatrolPoint
  (if (== (- (Utilities|Array|Length (Variables|Default|GetPatrolPoints)) 1) (Variables|Default|GetPatrolPointIndex))
    ;;[1 1 1] Start again at the first PatrolPoint or start counting backwards
    ;;;[1 1 1] Are we going to backtrack the PatrolPoints?
    (if (Variables|Default|GetReversePatrolPathWhenDone)
      (Variables|Default|SetCurrentlyGoingBackwards true)
      ;;;[1 1 1] Go to the previous PatrolPoint
      (Variables|Default|SetPatrolPointIndex (- (Variables|Default|GetPatrolPointIndex) 1))
      (else
        ;;;[1 1 1] Go to the first PatrolPoint
        (Variables|Default|SetPatrolPointIndex 0)))
    (else
      ;;[1 1 1] Count in the right direction, and check so we switch direction when vi hit zero
      ;;;[1 1 1] Are you going in backwards order?
      (if (Variables|Default|GetCurrentlyGoingBackwards)
        ;;;[1 1 1] Are we at index zero?
        (if (== (Variables|Default|GetPatrolPointIndex) 0)
          (Variables|Default|SetCurrentlyGoingBackwards false)
          ;;;[1 1 1] Go to the next PatrolPoint
          (Variables|Default|SetPatrolPointIndex (+ (Variables|Default|GetPatrolPointIndex) 1) :!label _label)
          (else
            ;;;[1 1 1] Go to the previous PatrolPoint
            (Variables|Default|SetPatrolPointIndex (- (Variables|Default|GetPatrolPointIndex) 1))))
        (else
          (goto _label))))))