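; Checkpoint actor that records itself as the player's active checkpoint and provides a respawn location.
; When bpPlayer overlaps the ActivationVolume, it shows its flag and loads or creates a bpCheckpointSave in the "Checkpoint" slot.
; It stores a reference to itself in that save and writes the slot back.
; GetPlayerSpawnLocation returns the world location of its PlayerSpawnLocation component.
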(event OnComponentBeginOverlap(ActivationVolume)
  (params (OverlappedComponent :type Primitive%20Component%20Object%20Reference) (OtherActor :type Actor%20Object%20Reference) (OtherComp :type Primitive%20Component%20Object%20Reference) (OtherBodyIndex :type Integer) (bFromSweep :type Boolean) (SweepResult :type Hit%20Result%20Structure%20%28by%20ref%29))
  (bind _self self)
  (Utilities|Casting|CastTobpPlayer OtherActor)
  (Rendering|SetVisibility (Variables|Default|GetFlag) true false)
  (bind _returnvalue (SaveGame|DoesSaveGameExist "Checkpoint"))
  (if _returnvalue
    (bind _returnvalue_2 (SaveGame|LoadGamefromSlot "Checkpoint"))
    (bind _asbp_checkpoint_save (Utilities|Casting|CastTobpCheckpointSave _returnvalue_2)
      (:then
        (Variables|/Game/Blueprints/Misc/bpCheckpointSave.bpCheckpointSave_C|SetCheckpoint _asbp_checkpoint_save _self)
        (SaveGame|SaveGametoSlot _asbp_checkpoint_save "Checkpoint" :!label _label))
      (:CastFailed
        (Development|PrintString "Cast failed in bpPlayer. Wrong type of save game")))
    (else
      (bind _returnvalue_3 (SaveGame|CreateSaveGameObject "/Game/Blueprints/Misc/bpCheckpointSave.bpCheckpointSave_C"))
      (Variables|/Game/Blueprints/Misc/bpCheckpointSave.bpCheckpointSave_C|SetCheckpoint _returnvalue_3 _self)
      (goto _label))))

(event EventBeginPlay)

(event Collision|EventActorBeginOverlap
  (params (OtherActor :type Actor%20Object%20Reference)))

(event EventTick
  (params (DeltaSeconds :type Float%20%28single-precision%29)))

(fn ConstructionScript)

(fn GetPlayerSpawnLocation
  (return (Transformation|GetWorldLocation (Variables|Default|GetPlayerSpawnLocation))))