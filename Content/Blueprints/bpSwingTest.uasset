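; Test actor that swings like a pendulum around HookLocation in the YZ plane while IsMoving is set.
; BeginPlay derives radius, start angle and an inverse-square radius scale; Tick integrates the angle with multi-stage predictor-corrector steps and decaying damping, ignoring DeltaSeconds, so motion is frame-rate dependent.
; A non-sweep sphere overlap stops the swing on the starting side, or weakly reverses it on the other.
; Tick prints debug values.
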(event OnComponentBeginOverlap(Sphere)
  (params (OverlappedComponent :type Primitive%20Component%20Object%20Reference) (OtherActor :type Actor%20Object%20Reference) (OtherComp :type Primitive%20Component%20Object%20Reference) (OtherBodyIndex :type Integer) (bFromSweep :type Boolean) (SweepResult :type Hit%20Result%20Structure%20%28by%20ref%29))
  (Variables|Default|SetHittedSomething? (not bFromSweep)))

(event EventBeginPlay
  (bind _returnvalue (Transformation|GetActorLocation))
  (bind _hooklocation (Variables|Default|GetHookLocation))
  (bind _returnvalue_2 (- _hooklocation _returnvalue))
  (Variables|Default|SetRadius (Math|Vector|VectorLength _returnvalue_2))
  ;[1 1 1] Fixa så den är oberoende av frame rate
  (Variables|Default|SetScaling (/ 3e+03 (Math|Float|Power (Variables|Default|GetRadius) 2.0)))
  (bind _output_get (Variables|Default|SetStartAngle (+ (Class|KismetMathLibrary|DegAcos (.y (Math|Vector|Normalize _returnvalue_2))) 9e+01)))
  (Variables|Default|SetTheta _output_get))

(event Collision|EventActorBeginOverlap
  (params (OtherActor :type Actor%20Object%20Reference)))

(event EventTick
  (params (DeltaSeconds :type Float%20%28single-precision%29))
  (bind _hooklocation (Variables|Default|GetHookLocation))
  (Development|PrintString (Utilities|String|Append "Theta: " (Utilities|String|ToString(Float) (Variables|Default|GetTheta))) true true "(R=1.000000,G=0.032634,B=0.000000,A=1.000000)" DeltaSeconds)
  (Development|PrintString (Utilities|String|Append "DTheta: " (Utilities|String|ToString(Float) (Variables|Default|GetdTheta))) true true "(R=1.000000,G=0.000000,B=0.000000,A=1.000000)" DeltaSeconds)
  (Development|PrintString (Utilities|String|Append "FirstDDTheta: " (Utilities|String|ToString(Float) (Variables|Default|GetFirstDDtheta))) true true "(R=1.000000,G=0.000000,B=0.054508,A=1.000000)" DeltaSeconds)
  (Development|PrintString (Utilities|String|Append "MidDDTheta: " (Utilities|String|ToString(Float) (Variables|Default|GetMidDDTheta))) true true "(R=1.000000,G=0.006725,B=0.000000,A=1.000000)" DeltaSeconds)
  (Development|PrintString (Utilities|String|Append "LastDDTheta: " (Utilities|String|ToString(Float) (Variables|Default|GetLastDDTheta))) true true "(R=1.000000,G=0.064177,B=0.000000,A=1.000000)" DeltaSeconds)
  (if (Variables|Default|GetisMoving?)
    ;[1 1 1] First
    (bind _output_get (Variables|Default|SetFirstDDtheta (* (Variables|Default|GetScaling) (* (Math|Trig|Sin(Degrees) (Variables|Default|GetTheta)) (Variables|Default|Gettest)))))
    (Variables|Default|SetMidDTheta (+ _output_get (Variables|Default|GetdTheta)))
    (Variables|Default|SetMidTheta (+ (Variables|Default|GetTheta) (/ (+ (Variables|Default|GetdTheta) (Variables|Default|GetMidDTheta)) 2.0)))
    ;[1 1 1] Second
    (Variables|Default|SetMidDDTheta (* (Variables|Default|GetScaling) (* (Math|Trig|Sin(Degrees) (Variables|Default|GetMidTheta)) (Variables|Default|Gettest))))
    (Variables|Default|SetMidDTheta (+ (Variables|Default|GetdTheta) (/ (+ (Variables|Default|GetFirstDDtheta) (Variables|Default|GetMidDDTheta)) 2.0)))
    (Variables|Default|SetMidTheta (+ (Variables|Default|GetTheta) (/ (+ (Variables|Default|GetdTheta) (Variables|Default|GetMidDTheta)) 2.0)))
    ;[1 1 1] Third
    (Variables|Default|SetMidDDTheta (* (Variables|Default|GetScaling) (* (Math|Trig|Sin(Degrees) (Variables|Default|GetMidTheta)) (Variables|Default|Gettest))))
    (Variables|Default|SetLastDTheta (+ (Variables|Default|GetMidDTheta) (Variables|Default|GetMidDDTheta)))
    (Variables|Default|SetLastTheta (+ (Variables|Default|GetMidTheta) (/ (+ (Variables|Default|GetMidDTheta) (Variables|Default|GetLastDTheta)) 2.0)))
    ;[1 1 1] Fourth
    (Variables|Default|SetLastDDTheta (* (Variables|Default|GetScaling) (* (Math|Trig|Sin(Degrees) (Variables|Default|GetLastTheta)) (Variables|Default|Gettest))))
    (Variables|Default|SetLastDTheta (+ (Variables|Default|GetMidDTheta) (/ (+ (Variables|Default|GetMidDDTheta) (Variables|Default|GetLastDDTheta)) 2.0)))
    (Variables|Default|SetLastTheta (+ (Variables|Default|GetMidTheta) (/ (+ (Variables|Default|GetMidDTheta) (Variables|Default|GetLastDTheta)) 2.0)))
    (Variables|Default|SetdTheta (* (Variables|Default|GetLastDTheta) (Variables|Default|GetDamping)))
    (Variables|Default|SetTheta (Variables|Default|GetLastTheta))
    ;[1 1 1] Fixa så den är obereoende av frame rate
    (Variables|Default|SetDamping (Math|Float|Clamp(Float) (- (Variables|Default|GetDamping) (/ 1.0 (Math|Float|Power (Variables|Default|GetRadius) 2.0)))))
    (Transformation|SetActorLocation (Math|Vector|MakeVector 0.0 (- (.y _hooklocation) (* (Variables|Default|GetRadius) (Math|Trig|Sin(Degrees) (Variables|Default|GetTheta)))) (+ (.z _hooklocation) (* (Variables|Default|GetRadius) (Math|Trig|Cos(Degrees) (Variables|Default|GetTheta))))) false false)
    (if (Variables|Default|GetHittedSomething?)
      (if (> (Variables|Default|GetStartAngle) 1.8e+02)
        (if (> (Variables|Default|GetTheta) 1.8e+02)
          (Variables|Default|SetisMoving? false :!label _label)
          (else
            (Variables|Default|SetdTheta (* (Variables|Default|GetdTheta) -0.01))
            (Variables|Default|SetDamping (* (Variables|Default|GetDamping) 0.99) :!label _label_2)
            (Variables|Default|SetHittedSomething? false)))
        (elif (<= (Variables|Default|GetTheta) 1.8e+02)
          (goto _label)
          (else
            (Variables|Default|SetdTheta (* (Variables|Default|GetdTheta) -0.01))
            (goto _label_2)))))))

(fn ConstructionScript)