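; Spawner actor that creates a row of enemies from its ActorsToSpawn class list when Activate is called.
; It spawns only when none of its previous enemies remain, offsetting each along world Y and skipping colliding placements.
; Each enemy receives the spawner as a reference and is tracked in EnemiesAlive until the EnemyDied event removes it, allowing another wave once the list empties.
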(event Custom|EnemyDied
  (params (Enemy :type Bp%20Enemy%20Base%20Object%20Reference))
  (Utilities|Array|RemoveItem (Variables|Default|GetEnemiesAlive) Enemy))

(event EventBeginPlay)

(event Collision|EventActorBeginOverlap
  (params (OtherActor :type Actor%20Object%20Reference)))

(event EventActivate
  (bind _returnvalue (Transformation|GetActorLocation))
  (bind _actorstospawn (Variables|Default|GetActorsToSpawn))
  ;[1 1 1] Don't spawn anything if there are enemies alive
  (if (== (Utilities|Array|Length (Variables|Default|GetEnemiesAlive)) 0)
    (for _index (range 0 (- (Utilities|Array|Length _actorstospawn) 1))
      (bind _returnvalue_2 (Game|SpawnActorfromClass (Utilities|Array|Get(acopy) _actorstospawn _index) (Math|Transform|MakeTransform (Math|Vector|MakeVector (.x _returnvalue) (+ (.y _returnvalue) (* _index -2.5e+02)) (.z _returnvalue))) "DontSpawnIfColliding" 0 self 0))
      (Utilities|Array|Add (Variables|Default|GetEnemiesAlive) _returnvalue_2))))

(event EventTick
  (params (DeltaSeconds :type Float%20%28single-precision%29)))

(fn ConstructionScript)