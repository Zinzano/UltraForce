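; Game mode that spawns and respawns the player at the last saved checkpoint, falling back to the first PlayerStart.
; GetSpawnLocation reads the Checkpoint save slot, creating an empty save if none exists, and also feeds the ChoosePlayerStart override.
; RespawnPlayer spawns a new BpPlayer at the checkpoint's spawn point or start actor's location, then possesses it with player controller 0 and disables its input.
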(event EventBeginPlay)

(event EventTick
  (params (DeltaSeconds :type Float%20%28single-precision%29)))

(fn ConstructionScript)

(fn ChoosePlayerStart
  (params (Player :type Controller%20Object%20Reference))
  (return (CallFunction|GetSpawnLocation)))

(fn RespawnPlayer
  (bind _returnvalue (Game|GetPlayerController 0))
  (bind _spawnactor (CallFunction|GetSpawnLocation))
  (bind _returnvalue_2 (Game|GetPlayerController 0))
  (bind _asbp_checkpoint (Utilities|Casting|CastTobpCheckpoint _spawnactor)
    (:then
      (bind _returnvalue_3 (Game|SpawnActorfromClass "/Game/Blueprints/Misc/bpPlayer.bpPlayer_C" (Math|Transform|MakeTransform (Default|GetPlayerSpawnLocation _asbp_checkpoint) "0, 0, 0" "1,1,1") "Undefined" 0 0))
      (Pawn|Possess _returnvalue _returnvalue_3)
      (Input|DisableInput _returnvalue_3 _returnvalue))
    (:CastFailed
      (bind _returnvalue_4 (Game|SpawnActorfromClass "/Game/Blueprints/Misc/bpPlayer.bpPlayer_C" (Math|Transform|MakeTransform (Transformation|GetActorLocation _spawnactor) "0, 0, 0" "1,1,1") "Undefined" 0 0))
      (Pawn|Possess _returnvalue_2 _returnvalue_4)
      (Input|DisableInput _returnvalue_4 _returnvalue_2))))

(fn GetSpawnLocation
  (bind _returnvalue (SaveGame|DoesSaveGameExist "Checkpoint"))
  (if _returnvalue
    (bind _returnvalue_2 (SaveGame|LoadGamefromSlot "Checkpoint"))
    (bind _asbp_checkpoint_save (Utilities|Casting|CastTobpCheckpointSave _returnvalue_2)
      (:then
        (if (Utilities|IsValid (Variables|/Game/Blueprints/Misc/bpCheckpointSave.bpCheckpointSave_C|GetCheckpoint _asbp_checkpoint_save))
          (return (Variables|/Game/Blueprints/Misc/bpCheckpointSave.bpCheckpointSave_C|GetCheckpoint _asbp_checkpoint_save))
          (else
            _)))
      (:CastFailed
        (Development|PrintString "Cast failed in bpPlayer. Wrong type of save game")))
    (else
      (bind _returnvalue_3 (SaveGame|CreateSaveGameObject "/Game/Blueprints/Misc/bpCheckpointSave.bpCheckpointSave_C"))
      (SaveGame|SaveGametoSlot _returnvalue_3 "Checkpoint")))
  (bind _outactors (Actor|GetAllActorsOfClass "/Script/Engine.PlayerStart"))
  (return (Utilities|Array|Get(acopy) _outactors)))