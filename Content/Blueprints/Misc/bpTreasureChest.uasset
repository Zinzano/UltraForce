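; Treasure chest actor that opens and spews random pickups when the player enters its activation volume.
; The first bpPlayer overlap plays the lid animation once, waits briefly, then starts a looping timer on SpawnTreasure.
; Each tick of that timer spawns a scaled-down random class from TypesOfTreasures and launches it in a randomized upward arc along the Arrow direction.
; The timer clears once NumberOfTreasures have spawned.
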(event OnComponentBeginOverlap(ActivationVolume)
  (params (OverlappedComponent :type Primitive%20Component%20Object%20Reference) (OtherActor :type Actor%20Object%20Reference) (OtherComp :type Primitive%20Component%20Object%20Reference) (OtherBodyIndex :type Integer) (bFromSweep :type Boolean) (SweepResult :type Hit%20Result%20Structure%20%28by%20ref%29))
  (Utilities|Casting|CastTobpPlayer OtherActor)
  (Utilities|FlowControl|DoOnce false
    (:Completed
      (Components|Animation|PlayAnimation (Variables|Default|GetChest) "/Game/Animations/Misc/Chest_Anim.Chest_Anim" false)
      (Utilities|FlowControl|Delay 1.5)
      (Utilities|Time|SetTimerbyFunctionName 0 "SpawnTreasure" 0.5 true))))

(event Custom|SpawnTreasure
  (bind _typesoftreasures (Variables|Default|GetTypesOfTreasures))
  (bind _arrow (Variables|Default|GetArrow))
  (bind _returnvalue (Game|SpawnActorfromClass (Utilities|Array|Get(acopy) _typesoftreasures (Math|Random|RandomIntegerinRange 0 (- (Utilities|Array|Length _typesoftreasures) 1))) (Math|Transform|MakeTransform (Transformation|GetWorldLocation (Variables|Default|GetTreasureSpawnPoint)) "0, 0, 0" "0.300000,0.300000,0.300000") "AlwaysSpawn" 0 0))
  (Physics|AddImpulse (Variables|/Game/Blueprints/Misc/Pickups/bpPickupBASE.bpPickupBASE_C|GetPickupMesh _returnvalue) (* (Math|Vector|Normalize (+ (+ (Math|Vector|GetForwardVector _arrow) (* (Math|Vector|GetRightVector _arrow) (Math|Random|RandomFloatinRange -1.0 1.0))) "0, 0,2.000000")) 7.5e+02) "None" true)
  (Variables|Default|SetCounter (+ (Variables|Default|GetCounter) 1))
  (if (>= (Variables|Default|GetCounter) (Variables|Default|GetNumberOfTreasures))
    (Utilities|Time|ClearTimerbyFunctionName 0 "SpawnTreasure")))

(event EventBeginPlay)

(event Collision|EventActorBeginOverlap
  (params (OtherActor :type Actor%20Object%20Reference)))

(event EventTick
  (params (DeltaSeconds :type Float%20%28single-precision%29)))

(fn ConstructionScript)