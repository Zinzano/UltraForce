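; Lava flow actor that grows along a spline once activated, damaging and knocking back any bpPlayer that hits it.
; The MoveLava timeline, timed by TotalMovementTime, drives a distance that moves a slightly flared front mesh along the spline.
; Behind it, spline mesh segments are spawned at runtime point by point, each stretching toward the front while thickening.
; The meshes are query-only and block a single custom trace channel.
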(event EventBeginPlay)

(event EventActivate
  (bind _meshcomp (CallFunction|GetMeshCompatCounter))
  (bind _counter (Variables|Default|Getcounter))
  (bind _counter_2 (Variables|Default|Getcounter))
  (bind _counter_3 (Variables|Default|Getcounter))
  (bind _counter_4 (Variables|Default|Getcounter))
  (bind (_location _tangent) (CallFunction|GetLocationandTangentfromSplinePoint _counter_4))
  (bind (_location_2 _tangent_2) (CallFunction|GetLocationandTangentfromSplinePoint _counter))
  (bind (_location_3 _tangent_3) (CallFunction|GetLocationandTangentfromSplinePoint _counter_2))
  (bind (_location_4 _tangent_4) (CallFunction|GetLocationandTangentfromSplinePoint _counter_3))
  (Utilities|FlowControl|DoOnce false
    (:Completed
      (Components|Timeline|SetPlayRate (Variables|Default|GetMove%20lava) (/ 1.0 (Variables|Default|GetTotalMovementTime)))
      (bind _returnvalue (CallFunction|CreateandAttachMesh))
      (Variables|Default|SetfrontMesh _returnvalue)
      (SplineMesh|SetStartandEnd (Variables|Default|GetfrontMesh) _location_4 _tangent_4 _location_4 _tangent_4 true :!class /Script/Engine.SplineMeshComponent)
      (SplineMesh|SetStartScale (Variables|Default|GetfrontMesh) "(X=1.000000,Y=1.000000)" true :!class /Script/Engine.SplineMeshComponent)
      (SplineMesh|SetEndScale (Variables|Default|GetfrontMesh) "(X=1.100000,Y=1.100000)" true :!class /Script/Engine.SplineMeshComponent)
      (bind _returnvalue_2 (CallFunction|CreateandAttachMesh))
      (Utilities|Array|Add (Variables|Default|GetSplineMeshes) _returnvalue_2)
      (SplineMesh|SetStartandEnd _returnvalue_2 _location_2 _tangent_2 _location_2 _tangent_2 true :!class /Script/Engine.SplineMeshComponent)
      (bind _distance (Timeline|Move%20lava PlayFromStart)
        (:Update
          (Variables|Default|SetLerpDistance (Math|Float|Lerp (Spline|GetDistanceAlongSplineatSplinePoint (Variables|Default|GetSpline) 0) (CallFunction|GetMaxDistance) _distance))
          (if (and (>= (Variables|Default|GetLerpDistance) (Spline|GetDistanceAlongSplineatSplinePoint (Variables|Default|GetSpline) (+ (Variables|Default|Getcounter) 1))) (< (Variables|Default|GetLerpDistance) (CallFunction|GetMaxDistance)))
            (Math|Integer|IncrementInt (Variables|Default|Getcounter)
              (:%20%20
                (Variables|Default|SetstartScale "(X=0.800000,Y=0.800000)")
                (bind _returnvalue_3 (CallFunction|CreateandAttachMesh))
                (Utilities|Array|Add (Variables|Default|GetSplineMeshes) _returnvalue_3)
                (SplineMesh|SetStartandEnd (CallFunction|GetMeshCompatCounter) _location_3 _tangent_3 _location_3 _tangent_3 true :!class /Script/Engine.SplineMeshComponent)
                (SplineMesh|SetStartScale _meshcomp (Variables|Default|GetstartScale) true :!class /Script/Engine.SplineMeshComponent)
                (SplineMesh|SetEndScale _meshcomp (Variables|Default|GetstartScale) true :!class /Script/Engine.SplineMeshComponent))))
          (SplineMesh|SetStartandEnd (Variables|Default|GetfrontMesh) (.Location (CallFunction|GetLocationandTangentfromDistance (Math|Float|Clamp(Float) (- (Variables|Default|GetLerpDistance) 1e+02) 0.0 (CallFunction|GetMaxDistance)))) (.Tangent (CallFunction|GetLocationandTangentfromDistance (Math|Float|Clamp(Float) (- (Variables|Default|GetLerpDistance) 1e+02) 0.0 (CallFunction|GetMaxDistance)))) (.Location (CallFunction|GetLocationandTangentfromDistance (Math|Float|Clamp(Float) (+ (Variables|Default|GetLerpDistance) 1e+02) 0.0 (CallFunction|GetMaxDistance)))) (.Tangent (CallFunction|GetLocationandTangentfromDistance (Math|Float|Clamp(Float) (+ (Variables|Default|GetLerpDistance) 1e+02) 0.0 (CallFunction|GetMaxDistance)))) true :!class /Script/Engine.SplineMeshComponent)
          (SplineMesh|SetStartandEnd (CallFunction|GetMeshCompatCounter) _location _tangent (.Location (CallFunction|GetLocationandTangentfromDistance (Math|Float|Clamp(Float) (+ (Variables|Default|GetLerpDistance) 8.0) 0.0 (CallFunction|GetMaxDistance)))) (.Tangent (CallFunction|GetLocationandTangentfromDistance (Math|Float|Clamp(Float) (+ (Variables|Default|GetLerpDistance) 8.0) 0.0 (CallFunction|GetMaxDistance)))) true :!class /Script/Engine.SplineMeshComponent)
          (Variables|Default|SetstartScale (Math|Vector2D|MakeVector2D (Math|Float|Clamp(Float) (+ (.x (Variables|Default|GetstartScale)) 0.01) 0.8) (Math|Float|Clamp(Float) (+ (.x (Variables|Default|GetstartScale)) 0.01) 0.8)))
          (SplineMesh|SetStartScale (CallFunction|GetMeshCompatCounter) (Variables|Default|GetstartScale) true :!class /Script/Engine.SplineMeshComponent)
          (SplineMesh|SetEndScale (CallFunction|GetMeshCompatCounter) (Variables|Default|GetstartScale) true :!class /Script/Engine.SplineMeshComponent))))))

(event Collision|EventHit
  (params (MyComp :type Primitive%20Component%20Object%20Reference) (Other :type Actor%20Object%20Reference) (OtherComp :type Primitive%20Component%20Object%20Reference) (bSelfMoved :type Boolean) (HitLocation :type Vector) (HitNormal :type Vector :default "0, 0, 0") (NormalImpulse :type Vector :default "0, 0, 0") (Hit :type Hit%20Result%20Structure%20%28by%20ref%29))
  (bind _asbp_player (Utilities|Casting|CastTobpPlayer Other))
  (Default|ApplyDamage _asbp_player (Variables|Default|GetDamage))
  (Utilities|IsValid _asbp_player
    (:Is%20Valid
      (Character|LaunchCharacter _asbp_player (* (Math|Vector|Normalize (- (Transformation|GetWorldLocation (Variables|/Game/Blueprints/Misc/bpPlayer.bpPlayer_C|GetCenterPoint _asbp_player)) HitLocation)) (Variables|Default|GetHitKickbackForce)) true true))))

(event EventTick
  (params (DeltaSeconds :type Float%20%28single-precision%29)))

(fn ConstructionScript)

(fn GetLocationandTangentfromSplinePoint
  (params (SplinePointIndex :type Integer))
  (bind _spline (Variables|Default|GetSpline))
  (return (Spline|GetLocationatSplinePoint _spline SplinePointIndex "Local") (Spline|GetTangentatSplinePoint _spline SplinePointIndex "Local")))

(fn GetMaxDistance
  (bind _spline (Variables|Default|GetSpline))
  (return (Spline|GetDistanceAlongSplineatSplinePoint _spline (- (Spline|GetNumberOfSplinePoints _spline) 1))))

(fn GetLocationandTangentfromDistance
  (params (Distance :type Float%20%28single-precision%29))
  (bind _spline (Variables|Default|GetSpline))
  (return (Spline|GetLocationatDistanceAlongSpline _spline Distance "Local") (Spline|GetTangentatDistanceAlongSpline _spline Distance "Local")))

(fn CreateandAttachMesh
  (bind _returnvalue (AddComponent|AddSplineMeshComponent false))
  (Components|StaticMesh|SetStaticMesh _returnvalue (Variables|Default|GetSplineMesh))
  (SplineMesh|SetForwardAxis _returnvalue (Variables|Default|GetForwardAxis) true)
  (Transformation|AttachComponentToComponent _returnvalue (Variables|Default|GetSpline) "None" "KeepRelative" "KeepRelative" "KeepRelative" true)
  (Collision|SetCollisionEnabled _returnvalue "QueryOnly")
  (Collision|SetCollisionResponsetoAllChannels _returnvalue "ECR_Ignore")
  (Collision|SetCollisionResponsetoChannel _returnvalue "ECC_GameTraceChannel1" "ECR_Block")
  (return _returnvalue))

(fn GetMeshCompatCounter
  (return (Utilities|Array|Get(acopy) (Variables|Default|GetSplineMeshes) (Variables|Default|Getcounter))))