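; Base projectile Blueprint that flies at a configurable speed and damages enemies on contact.
; The construction script applies Speed as both initial and max projectile movement speed and sets the projectile particle template.
; Any collision sphere overlap spawns a hit effect, applies Damage to the bpEnemy_Base cast result, and destroys the projectile, even when the cast fails.
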(event OnComponentBeginOverlap(CollisionSphere)
  (params (OverlappedComponent :type Primitive%20Component%20Object%20Reference) (OtherActor :type Actor%20Object%20Reference) (OtherComp :type Primitive%20Component%20Object%20Reference) (OtherBodyIndex :type Integer) (bFromSweep :type Boolean) (SweepResult :type Hit%20Result%20Structure%20%28by%20ref%29))
  ;[1 1 1] BeginOverlap
  (bind _asbp_enemy_base (Utilities|Casting|CastTobpEnemy_Base OtherActor)
    (:then
      _)
    (:CastFailed
      _))
  (Effects|SpawnEmitteratLocation (Variables|UL|GetPE_HittedSomething) (Transformation|GetActorLocation))
  (Game|Damage|ApplyDamage _asbp_enemy_base (Variables|UL|GetDamage) 0 0)
  (Actor|DestroyActor))

(event EventBeginPlay)

(event Collision|EventActorBeginOverlap
  (params (OtherActor :type Actor%20Object%20Reference)))

(event EventTick
  (params (DeltaSeconds :type Float%20%28single-precision%29)))

(fn ConstructionScript
  (bind _projectilemovement (Variables|Default|GetProjectileMovement))
  (bind _output_get (Variables|/Script/Engine.ProjectileMovementComponent|SetInitialSpeed _projectilemovement (Variables|UL|GetSpeed)))
  (Variables|/Script/Engine.ProjectileMovementComponent|SetMaxSpeed _projectilemovement _output_get)
  (Effects|Components|ParticleSystem|SetTemplate (Variables|Default|GetProjectileEffect) (Variables|UL|GetPE_Projectile)))