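; bpLavaFlow is an actor, named as a lava flow, that moves along Z at a set Speed once Activate is called.
; Tick advances the Z position each frame until the gap between EndHeight and the actor's Y coordinate is within a small tolerance, so the stop check ignores the axis being moved.
; The construction script also stores the Y coordinate as StartHeight, which the graphs shown never read.
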(event EventBeginPlay)

(event Collision|EventActorBeginOverlap
  (params (OtherActor :type Actor%20Object%20Reference)))

(event EventTick
  (params (DeltaSeconds :type Float%20%28single-precision%29))
  (bind _returnvalue (Transformation|GetActorLocation))
  (if (Variables|UltraForce|GetisMoving?)
    (if (<= (Math|Float|Absolute(Float) (- (Variables|UltraForce|GetEndHeight) (.y (Transformation|GetActorLocation)))) 3e+01)
      (Variables|UltraForce|SetisMoving? false)
      (else
        (Transformation|SetActorLocation (Math|Vector|MakeVector (.x _returnvalue) (.y _returnvalue) (+ (.z _returnvalue) (* DeltaSeconds (Variables|UltraForce|GetSpeed)))) false false)))))

(event EventActivate
  (Variables|UltraForce|SetisMoving? true))

(fn ConstructionScript
  (Variables|UltraForce|SetStartHeight (.y (Transformation|GetActorLocation))))