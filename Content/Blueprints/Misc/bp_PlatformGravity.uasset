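; bp_PlatformGravity is a physics-driven platform that dips when something overlaps its Box and is pushed back up toward its starting height.
; BeginPlay stores the start location and enables physics simulation on the StaticMesh.
; While below that height, Tick applies upward acceleration that scales with displacement via Force and Amplitude, like a spring.
; A Box overlap zeroes the mesh's velocity and applies a downward velocity-change impulse.
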(event OnComponentBeginOverlap(Box)
  (params (OverlappedComponent :type Primitive%20Component%20Object%20Reference) (OtherActor :type Actor%20Object%20Reference) (OtherComp :type Primitive%20Component%20Object%20Reference) (OtherBodyIndex :type Integer) (bFromSweep :type Boolean) (SweepResult :type Hit%20Result%20Structure%20%28by%20ref%29))
  (Physics|SetPhysicsLinearVelocity (Variables|Default|GetStaticMesh) "0, 0, 0" false "None")
  (Physics|AddImpulse (Variables|Default|GetStaticMesh) (* "0, 0,-1.000000" 2.5e+02) "None" true))

(event EventBeginPlay
  (Variables|Default|SetLocation (Transformation|GetActorLocation))
  (Physics|SetSimulatePhysics (Variables|Default|GetStaticMesh) true))

(event Collision|EventActorBeginOverlap
  (params (OtherActor :type Actor%20Object%20Reference)))

(event EventTick
  (params (DeltaSeconds :type Float%20%28single-precision%29))
  (if (> (.z (Variables|Default|GetLocation)) (.z (Transformation|GetActorLocation)))
    ;[1 1 1] Comment
    (Physics|AddForce (Variables|Default|GetStaticMesh) (* "0, 0,1.000000" (Math|Float|Lerp 0.0 (Variables|Default|GetForce) (/ (Math|Vector|VectorLength (- (Variables|Default|GetLocation) (Transformation|GetActorLocation))) (Variables|Default|GetAmplitude)))) "None" true)))

(fn ConstructionScript)