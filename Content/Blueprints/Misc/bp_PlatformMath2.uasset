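; Moving platform actor that travels one patrol-point leg each time the player lands on it, with a sine-driven landing bob on its mesh.
; The LandingArea overlap sets flags that Tick uses to run the bob and constant-speed movement.
; On arrival it stops and advances the patrol index, either wrapping or ping-ponging.
; Construction snaps it to the first point; an interpolated MovePlatform2 and timer-based logic are left unused.
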(event OnComponentBeginOverlap(LandingArea)
  (params (OverlappedComponent :type Primitive%20Component%20Object%20Reference) (OtherActor :type Actor%20Object%20Reference) (OtherComp :type Primitive%20Component%20Object%20Reference) (OtherBodyIndex :type Integer) (bFromSweep :type Boolean) (SweepResult :type Hit%20Result%20Structure%20%28by%20ref%29))
  ;[1 1 1] BeginOverlap
  (Utilities|Casting|CastTobpPlayer OtherActor)
  (if (not (Variables|Default|GetplayLandingAni?))
    (Variables|Default|SetplayLandingAni? true)
    (if (not (Variables|Default|GetisMoving?))
      (Variables|Default|SetisMoving? true))))

(event Custom|IncrementPP
  ;[1 1 1] IncrementPatrolPointIndex
  ;;[1 1 1] Are we at the last PatrolPoint
  (if (== (- (Utilities|Array|Length (Variables|UltraForce-Movement|GetPatrolPoints)) 1) (Variables|UltraForce-Movement|GetPatrolPointIndex))
    ;;[1 1 1] Start again at the first PatrolPoint or start counting backwards
    ;;;[1 1 1] Are we going to backtrack the PatrolPoints?
    (if (Variables|UltraForce-Movement|GetReversePatrolPathWhenDone)
      (Variables|UltraForce-Movement|SetCurrentlyGoingBackwards true)
      ;;;[1 1 1] Go to the previous PatrolPoint
      (Variables|UltraForce-Movement|SetPatrolPointIndex (- (Variables|UltraForce-Movement|GetPatrolPointIndex) 1))
      (else
        ;;;[1 1 1] Go to the first PatrolPoint
        (Variables|UltraForce-Movement|SetPatrolPointIndex 0)))
    (else
      ;;[1 1 1] Count in the right direction, and check so we switch direction when vi hit zero
      ;;;[1 1 1] Are you going in backwards order?
      (if (Variables|UltraForce-Movement|GetCurrentlyGoingBackwards)
        ;;;[1 1 1] Are we at index zero?
        (if (== (Variables|UltraForce-Movement|GetPatrolPointIndex) 0)
          (Variables|UltraForce-Movement|SetCurrentlyGoingBackwards false)
          ;;;[1 1 1] Go to the next PatrolPoint
          (Variables|UltraForce-Movement|SetPatrolPointIndex (+ (Variables|UltraForce-Movement|GetPatrolPointIndex) 1) :!label _label)
          (else
            ;;;[1 1 1] Go to the previous PatrolPoint
            (Variables|UltraForce-Movement|SetPatrolPointIndex (- (Variables|UltraForce-Movement|GetPatrolPointIndex) 1))))
        (else
          (goto _label))))))

(event Custom|LandingAnimation
  ;[1 1 1] LandingAnimation
  (if (>= (Variables|UltraForce-LandingAnimation|GetDegree2) 3.6e+02)
    (Variables|Default|SetplayLandingAni? false)
    (Variables|UltraForce-LandingAnimation|SetDegree2 1.8e+02)
    (Transformation|SetRelativeLocation (Variables|Default|GetStaticMesh) (Math|Vector|MakeVector 0.0 0.0 0.0) false false)
    (else
      (Transformation|SetRelativeLocation (Variables|Default|GetStaticMesh) (Math|Vector|MakeVector 0.0 0.0 (* (Math|Trig|Sin(Degrees) (Variables|UltraForce-LandingAnimation|GetDegree2)) (Variables|UltraForce-LandingAnimation|GetAmplitude))) false false)
      (Variables|UltraForce-LandingAnimation|SetDegree2 (+ (Variables|UltraForce-LandingAnimation|GetDegree2) (* (Variables|UltraForce-LandingAnimation|GetSpeed) (Variables|Default|GetDeltaSeconds)))))))

(event Custom|MovePlatform
  ;[1 1 1] MovePlatform
  (if (< (Math|Vector|VectorLength (- (Transformation|GetActorLocation) (CallFunction|GetTargetLocation))) 3e+01)
    (Variables|Default|SetisMoving? false)
    (CallFunction|IncrementPP)
    (else
      (Transformation|SetActorLocation (+ (Transformation|GetActorLocation) "0, 0, 0" (* (Math|Vector|Normalize (- (CallFunction|GetTargetLocation) (Transformation|GetActorLocation))) (* (Variables|Default|GetDeltaSeconds) (Variables|UltraForce-Movement|GetMovementSpeed)))) false false))))

(event Custom|MovePlatform2
  ;[1 1 1] MovePlatform2
  (if (< (Math|Vector|VectorLength (- (Transformation|GetActorLocation) (CallFunction|GetTargetLocation))) 3e+01)
    (Utilities|Time|ClearTimerbyFunctionName 0 "MovePlatform2")
    (CallFunction|IncrementPP)
    (else
      (Transformation|SetActorLocation (Math|Interpolation|VInterpTo (Transformation|GetActorLocation) (CallFunction|GetTargetLocation) (Variables|Default|GetDeltaSeconds) (Variables|UltraForce-Movement|GetMovementSpeed)) false false))))

(event EventBeginPlay
  ;[1 1 1] BeginPlay
)

(event Collision|EventActorBeginOverlap
  (params (OtherActor :type Actor%20Object%20Reference)))

(event EventTick
  (params (DeltaSeconds :type Float%20%28single-precision%29))
  ;[1 1 1] Tick
  (Variables|Default|SetDeltaSeconds DeltaSeconds)
  (if (Variables|Default|GetplayLandingAni?)
    (CallFunction|LandingAnimation))
  (if (Variables|Default|GetisMoving?)
    (CallFunction|MovePlatform)))

(fn ConstructionScript
  (bind _patrolpoints (Variables|UltraForce-Movement|GetPatrolPoints))
  (if (> (Utilities|Array|Length _patrolpoints) 0)
    (Transformation|SetActorLocation (Transformation|GetActorLocation (Utilities|Array|Get(acopy) _patrolpoints)) false false)))

(fn GetTargetLocation
  (bind _patrolpoints (Variables|UltraForce-Movement|GetPatrolPoints))
  (if (> (Utilities|Array|Length _patrolpoints) 0)
    (return (Transformation|GetActorLocation (Utilities|Array|Get(acopy) _patrolpoints (Variables|UltraForce-Movement|GetPatrolPointIndex))))
    (else
      (return (Transformation|GetActorLocation)))))